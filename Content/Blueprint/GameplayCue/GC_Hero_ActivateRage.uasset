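; Gameplay cue notify actor that provides the visual and audio feedback for the hero's activated rage.
; WhileActive spawns a Niagara activation effect and plays a cast sound at the target's location, and attaches a fire effect to the cue's target attach component.
; It stores that attached effect so OnRemove can destroy it when the cue ends.
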(fn `OnRemove`
  (params (MyTarget :type "Actor Object Reference") (Parameters :type "GameplayCueParameters Structure (by ref)"))
  (returns (ReturnValue :type Boolean))
  (bind _attachedrageeffect (`self.AttachedRageEffect`)
    (:`then`
      (`ActorComponent.K2_DestroyComponent` _attachedrageeffect null)
      (return false))
    (:`else`)))

(fn `UserConstructionScript`)

(fn `WhileActive`
  (params (MyTarget :type "Actor Object Reference") (Parameters :type "GameplayCueParameters Structure (by ref)"))
  (returns (ReturnValue :type Boolean))
  (`|ExecutionSequence`
    (:`then_0`
      (`NiagaraFunctionLibrary.SpawnSystemAtLocation` null "/Game/Assets/Niagara/Rage/NS_RageActivate.NS_RageActivate" (`self.K2_GetActorLocation` (`local.MyTarget`))))
    (:`then_1`
      (bind _returnvalue (`NiagaraFunctionLibrary.SpawnSystemAttached` "/Game/Assets/Niagara/Rage/NS_SampleSKFire.NS_SampleSKFire" (`.TargetAttachComponent` (`AbilitySystemBlueprintLibrary.BreakGameplayCueParameters` (`local.Parameters`))) "None" (0.0 0.0 0.0) (struct) "KeepRelativeOffset"))
      (set `self.AttachedRageEffect` _returnvalue))
    (:`then_2`
      (`GameplayStatics.PlaySoundAtLocation` null "/Game/Assets/Sounds/Abilities/SC_Ability_FireballCast.SC_Ability_FireballCast" (`self.K2_GetActorLocation` (`local.MyTarget`)) (struct) 1.0 1.0 0.0 null null null null))))