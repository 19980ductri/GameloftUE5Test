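; Gameplay ability that unequips the hero's rifle, apparently adapted from an axe version.
; It plays the axe unequip montage; a rifle unequip event attaches the rifle to the axe back socket and clears the equipped tag.
; HandleUnequipWeapon, fed the axe rather than the rifle, unlinks anim layers, removes input mapping and granted abilities, and refreshes weapon UI.
; The ability ends when the montage finishes or aborts.
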(event `self.K2_ActivateAbility`
  (set `self.CarriedWeapon` (`PawnCombatComponent.GetCarriedWeaponByTag` (`self.GetHeroCombatComponentFromActorInfo`) (struct :`TagName` "Player.Weapon.Axe")))
  (`AbilityTask_PlayMontageAndWait.CreatePlayMontageAndWaitProxy` "None" "/Game/Blueprint/PlayerCharacter/Montages/AM_Hero_Axe_Unequip.AM_Hero_Axe_Unequip"
    (:`then`
      (`AbilityTask_WaitGameplayEvent.WaitGameplayEvent` (struct :`TagName` "Player.Ability.Unequip.Rifle") null
        (:`EventReceived`
          (`Actor.K2_AttachToComponent` (`PawnCombatComponent.GetCarriedWeaponByTag` (`self.GetHeroCombatComponentFromActorInfo`) (struct :`TagName` "Player.Weapon.Rifle")) (`self.GetOwningComponentFromActorInfo`) "AxeBackSocket" "SnapToTarget" "KeepRelative" "KeepWorld" true)
          (`self.HandleUnequipWeapon` (`self.CarriedWeapon`))
          (set `PawnCombatComponent.CurrentEquippedWeaponTag` (struct) (`self.GetHeroCombatComponentFromActorInfo`)))))
    (:`OnCompleted`
      (`self.K2_EndAbility` :!label _label))
    (:`OnBlendOut`
      (goto _label))
    (:`OnInterrupted`
      (goto _label))
    (:`OnCancelled`
      (goto _label))))

(fn `HandleUnequipWeapon`
  (params (InWeapon :type "WarriorWeaponBase Object Reference"))
  (locals (CacedHeroWeaponData :type "WarriorHeroWeaponData Structure") (CachedGrantedAbilitySpec :type "Array of GameplayAbilitySpecHandle Structure"))
  (bind _cacedheroweapondata_weaponanimlayertolink (break `WarriorHeroWeaponData` (`local.CacedHeroWeaponData`)))
  (bind (_cacedheroweapondata_weaponanimlayertolink_2 _cacedheroweapondata_weaponinputmappingcontext) (break `WarriorHeroWeaponData` (`local.CacedHeroWeaponData`)))
  (bind _aswarrior_hero_weapon (cast `WarriorHeroWeapon` InWeapon))
  (set `local.CachedGrantedAbilitySpec` (`WarriorHeroWeapon.GetGrantedAbilitySpecHandles` _aswarrior_hero_weapon))
  (set `local.CacedHeroWeaponData` (`WarriorHeroWeapon.WeaponData` _aswarrior_hero_weapon))
  (`|ExecutionSequence`
    (:`then_0`
      (`SkeletalMeshComponent.UnlinkAnimClassLayers` (`self.GetOwningComponentFromActorInfo`) _cacedheroweapondata_weaponanimlayertolink))
    (:`then_1`
      (`EnhancedInputSubsystemInterface.RemoveMappingContext` (pcsubsystem `EnhancedInputLocalPlayerSubsystem` (`self.GetHeroControllerFromActorInfo`)) _cacedheroweapondata_weaponinputmappingcontext (struct))
      (`WarriorAbilitySystemComponent.RemoveGrantedHeroWeaponAbilities` (cast `WarriorAbilitySystemComponent` (`self.GetAbilitySystemComponentFromActorInfo`) :!pure true) (`local.CachedGrantedAbilitySpec`)))
    (:`then_2`
      (`HeroUIComponent.OnEquippedWeaponChanged` (`WarriorHeroCharacter.HeroUIComponent` (`self.GetHeroCharacterFromActorInfo`)) null)
      (for _array_element (`.SpecialWeaponAbilities` (break `WarriorHeroWeaponData` (`local.CacedHeroWeaponData`)))
        (`HeroUIComponent.OnAbilityIconSlotUpdated` (`WarriorHeroCharacter.HeroUIComponent` (`self.GetHeroCharacterFromActorInfo`)) (`.InputTag` (break `SpecialHeroAbilitySet` _array_element)) null)))))