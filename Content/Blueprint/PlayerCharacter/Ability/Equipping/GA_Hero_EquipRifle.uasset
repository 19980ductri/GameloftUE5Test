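; Hero gameplay ability that equips the carried rifle, setting it as the current weapon and attaching it to the WeaponRight socket.
; HandleEquipWeapon then uses its weapon data to link anim layers, add an input mapping context, and grant abilities, storing their handles on the weapon.
; It updates weapon and ability icons, restoring running cooldowns in the UI.
; Equipping is instant; the montage and gameplay-event wait are disconnected.
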(event `self.K2_ActivateAbility`
  (set `PawnCombatComponent.CurrentEquippedWeaponTag` (struct :`TagName` "Player.Weapon.Rifle") (`self.GetHeroCombatComponentFromActorInfo`))
  (`Actor.K2_AttachToComponent` (`PawnCombatComponent.GetCarriedWeaponByTag` (`self.GetHeroCombatComponentFromActorInfo`) (struct :`TagName` "Player.Weapon.Rifle")) (`self.GetOwningComponentFromActorInfo`) "WeaponRight" "SnapToTarget" "KeepRelative" "KeepWorld" true)
  (bind _returnvalue (`HeroCombatComponent.GetHeroCarriedWeaponByTag` (`self.GetHeroCombatComponentFromActorInfo`) (struct :`TagName` "Player.Weapon.Rifle")))
  (`self.HandleEquipWeapon` _returnvalue)
  (`self.K2_EndAbility`))

(event `self.K2_OnEndAbility`
  (params (bWasCancelled :type Boolean)))

(fn `HandleEquipWeapon`
  (params (InWeapon :type "WarriorHeroWeapon Object Reference"))
  (locals (CachedHeroWeaponData :type "WarriorHeroWeaponData Structure"))
  (bind (_cachedheroweapondata_weaponanimlayertolink _cachedheroweapondata_weaponinputmappingcontext _cachedheroweapondata_defaultweaponabilities _cachedheroweapondata_specialweaponabilities _cachedheroweapondata_weaponbasedamage _cachedheroweapondata_softweaponicon2d) (break `WarriorHeroWeaponData` (`local.CachedHeroWeaponData`)))
  (bind _cachedheroweapondata_weaponanimlayertolink_2 (break `WarriorHeroWeaponData` (`local.CachedHeroWeaponData`)))
  (bind (_cachedheroweapondata_weaponanimlayertolink_3 _cachedheroweapondata_weaponinputmappingcontext_2) (break `WarriorHeroWeaponData` (`local.CachedHeroWeaponData`)))
  (bind (_cachedheroweapondata_weaponanimlayertolink_4 _cachedheroweapondata_weaponinputmappingcontext_3 _cachedheroweapondata_defaultweaponabilities_2 _cachedheroweapondata_specialweaponabilities_2) (break `WarriorHeroWeaponData` (`local.CachedHeroWeaponData`)))
  (`KismetSystemLibrary.LogString` (`KismetSystemLibrary.GetObjectName` InWeapon))
  (set `local.CachedHeroWeaponData` (`WarriorHeroWeapon.WeaponData` InWeapon))
  (`|ExecutionSequence`
    (:`then_0`
      (`SkeletalMeshComponent.LinkAnimClassLayers` (`self.GetOwningComponentFromActorInfo`) _cachedheroweapondata_weaponanimlayertolink_2))
    (:`then_1`
      (`EnhancedInputSubsystemInterface.AddMappingContext` (pcsubsystem `EnhancedInputLocalPlayerSubsystem` (`self.GetHeroControllerFromActorInfo`)) _cachedheroweapondata_weaponinputmappingcontext_2 1 (struct)))
    (:`then_2`
      (bind _returnvalue (`WarriorAbilitySystemComponent.GrandWeaponAbilities` (`self.GetWarriorAbilitySystemComponentFromActorInfo`) _cachedheroweapondata_defaultweaponabilities_2 _cachedheroweapondata_specialweaponabilities_2 1))
      (`WarriorHeroWeapon.AssignGrantedAbilitySpecHandles` (`local.InWeapon`) _returnvalue))
    (:`then_3`
      (`HeroUIComponent.OnEquippedWeaponChanged` (`WarriorHeroCharacter.HeroUIComponent` (`self.GetHeroCharacterFromActorInfo`)) _cachedheroweapondata_softweaponicon2d)
      (for _array_element _cachedheroweapondata_specialweaponabilities
        (bind (_softabilityiconmaterial _abilitycooldowntag _inputtag) (break `SpecialHeroAbilitySet` _array_element))
        (`HeroUIComponent.OnAbilityIconSlotUpdated` (`WarriorHeroCharacter.HeroUIComponent` (`self.GetHeroCharacterFromActorInfo`)) _inputtag _softabilityiconmaterial)
        (bind (_totalcooldowntime _remaincooldowntime _returnvalue_2) (`self.GetAbilityRemainCooldownByTag` _abilitycooldowntag))
        (if _returnvalue_2
          (`HeroUIComponent.OnAbilityCooldownBegin` (`WarriorHeroCharacter.HeroUIComponent` (`self.GetHeroCharacterFromActorInfo`)) _inputtag _totalcooldowntime _remaincooldowntime))))))