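; Axe heavy attack gameplay ability for the hero, adding a slash projectile while rage is active.
; WhileRageActive waits for the SpawnProjectile gameplay event, then spawns BP_Projectile_HeroSlash at the equipped weapon's RageSlashSocket.
; The projectile takes its yaw from the hero's forward vector and roll from the socket.
; It carries a damage spec built from weapon damage, the Heavy attack tag and combo count.
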(event `self.WhileRageActive`
  (bind _returnvalue (`self.GetHeroCharacterFromActorInfo`))
  (bind (_returnvalue_roll _returnvalue_pitch _returnvalue_yaw) (`KismetMathLibrary.BreakRotator` (`KismetMathLibrary.MakeRotFromX` (`Actor.GetActorForwardVector` (`self.GetHeroCharacterFromActorInfo`)))))
  (bind _returnvalue_2 (`SceneComponent.GetSocketTransform` (`WarriorWeaponBase.WeaponMesh` (`HeroCombatComponent.GetHeroCurrentEquippedWeapon` (`self.GetHeroCombatComponentFromActorInfo`))) "RageSlashSocket" "RTS_World"))
  (`AbilityTask_WaitGameplayEvent.WaitGameplayEvent` (struct :`TagName` "Shared.Event.SpawnProjectile") null
    (:`EventReceived`
      (`|SpawnActorFromClass` "/Game/Blueprint/PlayerCharacter/BP_Projectile_HeroSlash.BP_Projectile_HeroSlash_C" (`KismetMathLibrary.MakeTransform` (.location _returnvalue_2) (`KismetMathLibrary.MakeRotator` (.roll (.rotation _returnvalue_2)) 0.0 _returnvalue_yaw)) "AdjustIfPossibleButAlwaysSpawn" "MultiplyWithRoot" _returnvalue (`self.MakeHeroDamageEffectSpecHandle` "/Game/Shared/GameplayEffects/GE_Shared_DealDamage.GE_Shared_DealDamage_C" (`HeroCombatComponent.GetHeroCurrentEquipWeaponDamageAtLevel` (`self.GetHeroCombatComponentFromActorInfo`) 0.0) (struct :`TagName` "Player.SetByCaller.AttackType.Heavy") (`self.UsedComboCount`)) _returnvalue))))