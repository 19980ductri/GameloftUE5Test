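; Master gameplay ability for the hero's heavy attack combo, playing a montage per combo step from a map.
; The JumpToFinisher tag skips to the last step; the count resets after the finisher or on a short timer after the ability ends.
; Melee hit events play a sound cue and apply combo-scaled SetByCaller damage, triggering hit react and rage gain on success.
; Active rage calls WhileRageActive, an empty hook here.
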(event `self.K2_ActivateAbility`
  ;[1 1 1] to make sure current count never equals to "0"
  (if (== (`self.CurrentHeavyAttackComboCount`) 0)
    (set `self.CurrentHeavyAttackComboCount` 1))
  (`KismetSystemLibrary.K2_ClearAndInvalidateTimerHandle` (`self.ComboResetTimerHandle`))
  (`WarriorFunctionLibrary.BP_DoesActorHaveTag` (`self.GetHeroCharacterFromActorInfo`) (struct :`TagName` "Player.Status.JumpToFinisher")
    (:`Yes`
      (set `self.CurrentHeavyAttackComboCount` (`BlueprintMapLibrary.Map_Length` (`self.AttackMontagesMap`))))
    (:`No`
      (`KismetSystemLibrary.PrintString` (`KismetStringLibrary.Conv_IntToString` (`self.CurrentHeavyAttackComboCount`)))))
  (set `self.UsedComboCount` (`self.CurrentHeavyAttackComboCount`))
  (`AbilityTask_PlayMontageAndWait.CreatePlayMontageAndWaitProxy` "None" (`BlueprintMapLibrary.Map_Find` (`self.AttackMontagesMap`) (`self.CurrentHeavyAttackComboCount`))
    (:`then`
      (`|ExecutionSequence`
        (:`then_0`
          ; Handle dmg
          (bind (_asynctaskproxy _payload) (`AbilityTask_WaitGameplayEvent.WaitGameplayEvent` (struct :`TagName` "Shared.Event.MeleeHit") null)
            (:`EventReceived`
              (`self.HandleApplyDamage` _payload))))
        (:`then_1`
          ; Combo Count
          (if (== (`self.CurrentHeavyAttackComboCount`) (`BlueprintMapLibrary.Map_Length` (`self.AttackMontagesMap`)))
            (`self.ResetAttackComboCount`)
            (else
              (`/Engine/EditorBlueprintResources/StandardMacros.IncrementInt` (`self.CurrentHeavyAttackComboCount`)))))
        (:`then_2`
          (`WarriorFunctionLibrary.BP_DoesActorHaveTag` (`self.GetHeroCharacterFromActorInfo`) (struct :`TagName` "Player.Status.Rage.Active")
            (:`Yes`
              (`self.WhileRageActive`))))))
    (:`OnCompleted`
      (`self.K2_EndAbility` :!label _label)
      (bind _returnvalue (`KismetSystemLibrary.K2_SetTimerDelegate` (delegate `ResetAttackComboCount`) 0.5))
      (set `self.ComboResetTimerHandle` _returnvalue))
    (:`OnBlendOut`
      (goto _label))
    (:`OnInterrupted`
      (goto _label))
    (:`OnCancelled`
      (goto _label))))

(event `WhileRageActive`)

(event `ResetAttackComboCount`
  (set `self.CurrentHeavyAttackComboCount` 1)
  (`WarriorFunctionLibrary.RemoveGameplayTagIfFound` (`self.GetHeroCharacterFromActorInfo`) (struct :`TagName` "Player.Status.JumpToFinisher")))

(event `self.K2_OnEndAbility`
  (params (bWasCancelled :type Boolean)))

(fn `HandleApplyDamage`
  (params (GameplayEventData :type "GameplayEventData Structure (by ref)"))
  (locals (LocalTarget :type "Actor Object Reference"))
  (bind _output_get (set `local.LocalTarget` (`.Target` (break `GameplayEventData` GameplayEventData))))
  (`self.K2_ExecuteGameplayCue` (`self.WeaponHitSoundGameplayCueTag`))
  (`self.BP_ApplyEffectSpecHandleToTarget` _output_get (`self.MakeHeroDamageEffectSpecHandle` "/Game/Shared/GameplayEffects/GE_Shared_DealDamage.GE_Shared_DealDamage_C" (`HeroCombatComponent.GetHeroCurrentEquipWeaponDamageAtLevel` (`self.GetHeroCombatComponentFromActorInfo`) (`KismetMathLibrary.Conv_IntToDouble` (`self.GetAbilityLevel`))) (struct :`TagName` "Player.SetByCaller.AttackType.Heavy") (`self.UsedComboCount`))
    (:`Successful`
      (`AbilitySystemBlueprintLibrary.SendGameplayEventToActor` (`local.LocalTarget`) (struct :`TagName` "Shared.Event.HitReact") (`local.GameplayEventData`))
      (`self.BP_ApplyGameplayEffectToOwner` "/Game/Blueprint/PlayerCharacter/GameplayEffect/GE_Hero_GainRage.GE_Hero_GainRage_C" (`self.GetAbilityLevel`)))))