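; Base enemy character Blueprint that handles dissolve effects on spawn and death.
; BeginPlay reverses a timeline driving the mesh's DissolveAmount to materialize the enemy and plays a random entry montage.
; OnEnemyDied freezes animation, disables capsule collision, removes UI, async-loads Niagara particles tinted from the material's edge color and dissolves the mesh.
; Afterwards it destroys weapon and actor, only if a weapon is valid; weapon dissolve nodes are disconnected.
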(event `self.ReceiveBeginPlay`
  (bind _entry_anim_montages (`self.Entry Anim Montages`))
  (`|ExecutionSequence`
    (:`then_0`
      (`TimelineComponent.SetPlayRate` (`self.Entry restore time line`) (/ 1.0 (`self.TotalEntryRestoreTime`)))
      (bind (_direction _normalizedfloattrack) (`Timeline|Entry restore time line` :!via `ReverseFromEnd`)
        (:`Update`
          (`MeshComponent.SetScalarParameterValueOnMaterials` (`self.Mesh`) "DissolveAmount" _normalizedfloattrack)
          (`/Engine/EditorBlueprintResources/StandardMacros.IsValid` (`PawnCombatComponent.GetCurrentEquippedWeapon` (`self.EnemyCombatComponent`))))))
    (:`then_1`
      (if (`KismetArrayLibrary.Array_IsNotEmpty` _entry_anim_montages)
        (`self.PlayAnimMontage` (`KismetArrayLibrary.Array_Random` _entry_anim_montages))))))

(event `/Game/Blueprint/Enemy/BPI_Enemy_Death.OnEnemyDied`
  (params (DissolveNiagaraSystem :type "NiagaraSystem Soft Object Reference"))
  (bind _mesh (`self.Mesh`))
  (bind _returnvalue (`PawnCombatComponent.GetCurrentEquippedWeapon` (`self.EnemyCombatComponent`)))
  (`|ExecutionSequence`
    (:`then_0`
      (set `SkeletalMeshComponent.bPauseAnims` true (`self.Mesh`))
      (`PrimitiveComponent.SetCollisionEnabled` (`self.CapsuleComponent`) "NoCollision"))
    (:`then_1`
      (`EnemyUIComponent.RemoveEnemyDrawnWidget` (`self.EnemyUIComponent`)))
    (:`then_2`
      (bind _object (`|LoadAsset` DissolveNiagaraSystem)
        (:`Completed`
          (bind _asniagara_system (cast `NiagaraSystem` _object))
          (bind _returnvalue_2 (`NiagaraFunctionLibrary.SpawnSystemAttached` _asniagara_system (`self.Mesh`) "None" (0.0 0.0 0.0) (struct) "KeepRelativeOffset"))
          (bind _returnvalue_3 (`PrimitiveComponent.CreateDynamicMaterialInstance` _mesh 0 (`PrimitiveComponent.GetMaterial` _mesh 0) "None"))
          (bind _returnvalue_4 (`MaterialInstanceDynamic.K2_GetVectorParameterValue` _returnvalue_3 "DissolveEdgeColor"))
          (`NiagaraComponent.SetNiagaraVariableLinearColor` _returnvalue_2 "DissolveParticleColor" _returnvalue_4)
          (`TimelineComponent.SetPlayRate` (`self.DissolveTime`) (/ 1.0 (`self.TotalDissovleTime`)))
          (bind (_direction _normalizedfloattrack) (`Timeline|DissolveTime` :!via `PlayFromStart`)
            (:`Update`
              (`MeshComponent.SetScalarParameterValueOnMaterials` (`self.Mesh`) "DissolveAmount" _normalizedfloattrack)
              (`/Engine/EditorBlueprintResources/StandardMacros.IsValid` (`PawnCombatComponent.GetCurrentEquippedWeapon` (`self.EnemyCombatComponent`))))
            (:`Finished`
              (`/Engine/EditorBlueprintResources/StandardMacros.IsValid` _returnvalue
                (:`Is Valid`
                  (`self.K2_DestroyActor` _returnvalue)
                  (`self.K2_DestroyActor`))))))))))

(fn `UserConstructionScript`)